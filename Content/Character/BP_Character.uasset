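; Player character for a lantern game in which the player lights candles before fuel runs out, managing title, oil and result widgets.
; Tick drains fuel per frame without delta-time scaling, showing the result screen at empty fuel or five lit candles.
; A Box overlap caches nearby candles or handlights for the Light input to trigger, counting each candle once.
; The Lantern input toggles the child-actor lantern, draining fuel faster while it burns.
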(event OnComponentBeginOverlap(Box)
  (params (OverlappedComponent :type Primitive%20Component%20Object%20Reference) (OtherActor :type Actor%20Object%20Reference) (OtherComp :type Primitive%20Component%20Object%20Reference) (OtherBodyIndex :type Integer) (bFromSweep :type Boolean) (SweepResult :type Hit%20Result%20Structure%20%28by%20ref%29))
  (Utilities|FlowControl|Sequence
    (:then_0
      (bind _asbp_candle_01 (Utilities|Casting|CastToBP_Candle_01 OtherActor))
      (Variables|Default|SetAs%20BP%20Candle%2001 _asbp_candle_01))
    (:then_1
      (bind _asbp_candle_02 (Utilities|Casting|CastToBP_Candle_02 OtherActor))
      (Variables|Default|SetAs%20BP%20Candle%2002 _asbp_candle_02))
    (:then_2
      (bind _asbp_handlight (Utilities|Casting|CastToBP_Handlight OtherActor))
      (Variables|Default|SetAs%20BP%20Handlight _asbp_handlight)
      (Development|PrintString "check"))))

(event OnComponentEndOverlap(Box)
  (params (OverlappedComponent :type Primitive%20Component%20Object%20Reference) (OtherActor :type Actor%20Object%20Reference) (OtherComp :type Primitive%20Component%20Object%20Reference) (OtherBodyIndex :type Integer))
  (Utilities|FlowControl|Sequence
    (:then_0
      (Utilities|Casting|CastToBP_Candle_01 OtherActor)
      (Variables|Default|SetAs%20BP%20Candle%2001 0)
      (Development|PrintString "E_Light01"))
    (:then_1
      (Utilities|Casting|CastToBP_Candle_02 OtherActor)
      (Variables|Default|SetAs%20BP%20Candle%2002 0)
      (Development|PrintString "E_Light02"))
    (:then_2
      (Utilities|Casting|CastToBP_Handlight OtherActor)
      (Variables|Default|SetAs%20BP%20Handlight 0))))

(event Input|EnhancedActionEvents|EnhancedInputActionIA_Lantern
  (params (ActionValue :type Boolean) (ElapsedSeconds :type Float%20%28double-precision%29) (TriggeredSeconds :type Float%20%28double-precision%29) (InputAction :type Input%20Action%20Object%20Reference :default "/Game/Buleprint/IA_Lantern.IA_Lantern"))
  (bind _as_bp_lantern (Variables|Default|GetAs%20BP%20Lantern))
  (:Started
    (Utilities|FlowControl|FlipFlop
      (:A
        (Default|OnBurning _as_bp_lantern)
        (Variables|Default|Setdown_fuel 2))
      (:B
        (Default|OffBurning _as_bp_lantern)
        (Variables|Default|Setdown_fuel 1)))))

(event Input|EnhancedActionEvents|EnhancedInputActionIA_Light
  (params (ActionValue :type Boolean) (ElapsedSeconds :type Float%20%28double-precision%29) (TriggeredSeconds :type Float%20%28double-precision%29) (InputAction :type Input%20Action%20Object%20Reference :default "/Game/Buleprint/IA_Light.IA_Light"))
  (bind _as_bp_candle_01 (Variables|Default|GetAs%20BP%20Candle%2001))
  (bind _as_bp_candle_02 (Variables|Default|GetAs%20BP%20Candle%2002))
  (bind _as_bp_handlight (Variables|Default|GetAs%20BP%20Handlight))
  (Utilities|FlowControl|Sequence
    (:then_0
      (Utilities|IsValid _as_bp_candle_01
        (:Is%20Valid
          (Default|OnLight _as_bp_candle_01)
          (if (not (Variables|/Game/Assets/BluePrint/BP_Candle_01.BP_Candle_01_C|GetbLight (Variables|Default|GetAs%20BP%20Candle%2001)))
            (Variables|Default|Setfire_count (+ (Variables|Default|Getfire_count) 1))
            (Default|Fire (Variables|Default|GetWBP_Oil))
            (Variables|/Game/Assets/BluePrint/BP_Candle_01.BP_Candle_01_C|SetbLight (Variables|Default|GetAs%20BP%20Candle%2001) true)))))
    (:then_1
      (Utilities|IsValid _as_bp_candle_02
        (:Is%20Valid
          (Default|OnLight _as_bp_candle_02)
          (if (not (Variables|/Game/Assets/BluePrint/BP_Candle_02.BP_Candle_02_C|GetbLight (Variables|Default|GetAs%20BP%20Candle%2002)))
            (Variables|Default|Setfire_count (+ (Variables|Default|Getfire_count) 1))
            (Default|Fire (Variables|Default|GetWBP_Oil))
            (Variables|/Game/Assets/BluePrint/BP_Candle_02.BP_Candle_02_C|SetbLight (Variables|Default|GetAs%20BP%20Candle%2002) true)))))
    (:then_2
      (Utilities|IsValid _as_bp_handlight
        (:Is%20Valid
          (Default|OnFrash _as_bp_handlight)
          (Development|PrintString "ON"))))))

(event EventBeginPlay
  (bind _asbp_lantern (Utilities|Casting|CastToBP_Lantern (Variables|/Script/Engine.ChildActorComponent|GetChildActor (Variables|Default|GetBP_Lantern))))
  (Variables|Default|SetAs%20BP%20Lantern _asbp_lantern)
  (bind _returnvalue (UserInterface|CreateWidget "/Game/UI/WBP_Title.WBP_Title_C"))
  (bind _output_get (Variables|Default|SetWBP_Title _returnvalue))
  (UserInterface|Viewport|AddtoViewport _output_get 0)
  (bind _returnvalue_2 (UserInterface|CreateWidget "/Game/UI/WBP_Oil.WBP_Oil_C"))
  (Variables|Default|SetWBP_Oil _returnvalue_2)
  (bind _returnvalue_3 (UserInterface|CreateWidget "/Game/UI/WBP_Result.WBP_Result_C"))
  (Variables|Default|SetWBP_Result _returnvalue_3))

(event Collision|EventActorBeginOverlap
  (params (OtherActor :type Actor%20Object%20Reference)))

(event EventTick
  (params (DeltaSeconds :type Float%20%28single-precision%29))
  (Utilities|FlowControl|Sequence
    (:then_0
      ;[0.15 0.15 0.15 0.5] 燃料の減少
      (if (Variables|Default|Getstart_in_game)
        (Variables|Default|Setnow_fuel (- (Variables|Default|Getnow_fuel) (Variables|Default|Getdown_fuel)))
        (if (not (> (Variables|Default|Getnow_fuel) 0))
          ;[0.15 0.15 0.15 0.5] Game over
          (Variables|Default|Setstart_in_game false)
          (Widget|RemovefromParent (Variables|Default|GetWBP_Oil))
          (UserInterface|Viewport|AddtoViewport (Variables|Default|GetWBP_Result) 0))))
    (:then_1
      ;[0.15 0.15 0.15 0.5] Game clear
      (if (>= (Variables|Default|Getfire_count) 5)
        (Variables|Default|Setstart_in_game false)
        (Widget|RemovefromParent (Variables|Default|GetWBP_Oil))
        (UserInterface|Viewport|AddtoViewport (Variables|Default|GetWBP_Result) 0)))
    (:then_2
      ;[0.15 0.15 0.15 0.5] In game
      (if (Variables|Default|Getstart_in_game)
        (Widget|RemovefromParent (Variables|Default|GetWBP_Title))
        (UserInterface|Viewport|AddtoViewport (Variables|Default|GetWBP_Oil) 0)))))

(fn ConstructionScript)