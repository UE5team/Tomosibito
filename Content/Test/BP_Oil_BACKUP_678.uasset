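; BP_Oil is a fuel pickup, saved here as a backup in a Test folder, that refills the player character's fuel.
; BeginPlay casts player 0's character to BP_Character and caches it.
; Any overlap on its Sphere component, without checking the overlapping actor, adds the cached character's MaxFuel to NowFuel, clamped to MaxFuel, then destroys the pickup.
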(event OnComponentBeginOverlap(Sphere)
  (params (OverlappedComponent :type Primitive%20Component%20Object%20Reference) (OtherActor :type Actor%20Object%20Reference) (OtherComp :type Primitive%20Component%20Object%20Reference) (OtherBodyIndex :type Integer) (bFromSweep :type Boolean) (SweepResult :type Hit%20Result%20Structure%20%28by%20ref%29))
  (bind _character (Variables|Default|GetCharacter))
  (bind _character_2 (Variables|Default|GetCharacter))
  (Variables|/Game/Character/BP_Character.BP_Character_C|Setnow_fuel _character (Math|Integer|Clamp(Integer) (+ (Variables|/Game/Character/BP_Character.BP_Character_C|Getnow_fuel _character_2) (Variables|/Game/Character/BP_Character.BP_Character_C|Getmax_fuel _character_2)) 0 (Variables|/Game/Character/BP_Character.BP_Character_C|Getmax_fuel _character)))
  (Actor|DestroyActor))

(event EventBeginPlay
  (bind _asbp_character (Utilities|Casting|CastToBP_Character (Game|GetPlayerCharacter 0)))
  (Variables|Default|SetCharacter _asbp_character))

(event EventTick
  (params (DeltaSeconds :type Float%20%28single-precision%29)))

(event Collision|EventActorBeginOverlap
  (params (OtherActor :type Actor%20Object%20Reference)))

(fn ConstructionScript)