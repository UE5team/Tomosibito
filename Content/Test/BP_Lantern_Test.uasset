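; Test lantern Blueprint that burns a fuel supply and lets the player try to light a lamp.
; Fuel starts at MaxFuel and drops by one each Tick until empty, so the burn rate depends on frame rate.
; Pressing E calls TryIgniteLamp with BPLamp, then with itself.
; OnExtinguish, meant for empty fuel, prints a game-over message, but nothing in this graph calls it.
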(event EventBeginPlay
  (Variables|Default|Setfuel (Variables|Default|Getmax_fuel)))

(event Collision|EventActorBeginOverlap
  (params (OtherActor :type Actor%20Object%20Reference)))

(event EventTick
  (params (DeltaSeconds :type Float%20%28single-precision%29))
  (if (> (Variables|Default|Getfuel) 0)
    (Variables|Default|Setfuel (- (Variables|Default|Getfuel) 1))))

(event EventOnExtinguish
  ;[0.15 0.15 0.15 0.5] 燃料が０になったら発火するイベント
  (Development|PrintString "game over"))

(event Input|KeyboardEvents|E
  (params (Key :type Key%20Structure :default "None"))
  (:Pressed
    ;[0.15 0.15 0.15 0.5] ランプに火を灯せるか確認。灯せるならランプに通知
    (Class|Lantern|TryIgniteLamp (Variables|Default|GetBP_Lamp))
    (Class|Lantern|TryIgniteLamp self)))

(fn ConstructionScript)