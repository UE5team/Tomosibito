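; BP_Candle_02 is a candle actor with a point light that starts hidden and can be switched on or off.
; The OnLight and OffLight events toggle the light's visibility, while Tick reapplies the IntensityLight and RadiusLight variables to it every frame.
; BeginPlay caches the player's BP_Character, but the only logic using it, a FireCount increment, is disconnected.
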(event Custom|OnLight
  (Rendering|SetVisibility (Variables|Default|GetPointLight) true true))

(event Custom|OffLight
  (Rendering|SetVisibility (Variables|Default|GetPointLight) false true))

(event EventBeginPlay
  (Rendering|SetVisibility (Variables|Default|GetPointLight) false true)
  (bind _asbp_character (Utilities|Casting|CastToBP_Character (Game|GetPlayerCharacter 0)))
  (Variables|Default|SetCharacter _asbp_character))

(event Collision|EventActorBeginOverlap
  (params (OtherActor :type Actor%20Object%20Reference)))

(event EventTick
  (params (DeltaSeconds :type Float%20%28single-precision%29))
  (bind _pointlight (Variables|Default|GetPointLight))
  (Rendering|Components|Light|SetIntensity _pointlight (Variables|Default|GetIntensityLight))
  (Rendering|Lighting|SetAttenuationRadius _pointlight (Variables|Default|GetRadiusLight)))

(fn ConstructionScript)