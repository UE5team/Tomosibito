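; BP_Handlight is a hand light built on a spotlight, whose starting visibility comes from the Light variable.
; Every Tick it copies the Intensity, Distance and CornRadius variables onto the spotlight, deriving the inner cone angle as a fixed fraction of the outer.
; The onFrash event blinks the light off for FlashTime, then always switches it back on, regardless of Light.
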(event Custom|onFrash
  (bind _spotlight (Variables|Default|GetSpotLight))
  (Rendering|SetVisibility _spotlight false true)
  (Utilities|FlowControl|Delay (Variables|Default|GetFlashTime))
  (Rendering|SetVisibility _spotlight true true))

(event EventBeginPlay
  (Rendering|SetVisibility (Variables|Default|GetSpotLight) (Variables|Default|GetbLight) true))

(event Collision|EventActorBeginOverlap
  (params (OtherActor :type Actor%20Object%20Reference)))

(event EventTick
  (params (DeltaSeconds :type Float%20%28single-precision%29))
  (bind _spotlight (Variables|Default|GetSpotLight))
  (bind _cornradius (Variables|Default|GetCornRadius))
  (Rendering|Components|Light|SetIntensity _spotlight (Variables|Default|GetIntensity))
  (Rendering|Lighting|SetAttenuationRadius _spotlight (Variables|Default|GetDistance))
  (Rendering|Lighting|SetOuterConeAngle _spotlight _cornradius)
  (Rendering|Lighting|SetInnerConeAngle _spotlight (* _cornradius 0.8)))

(fn ConstructionScript)